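; Spline-following moving platform actor that starts moving on BeginPlay.
; A timeline, played at the Rate variable's speed, outputs a normalized SplineDistance that is scaled by spline length to set the mesh's world location along the spline.
; Movement is unswept and leaves rotation untouched.
; The construction script applies the configurable static mesh and material to the platform.
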(event `self.ReceiveBeginPlay`
  (`self.Platform Start`))

(event `Platform Start`
  (bind _spline (`self.Spline`))
  (`TimelineComponent.SetPlayRate` (`self.Motion Timeline`) (`self.Rate`))
  (bind (_direction _spline_distance) (`Timeline|Motion Timeline`)
    (:`Update`
      (`SceneComponent.K2_SetWorldLocation` (`self.PlatformMesh`) (`SplineComponent.GetLocationAtDistanceAlongSpline` _spline (* _spline_distance (`SplineComponent.GetSplineLength` _spline)) "World") false false))))

(fn `UserConstructionScript`
  (bind _platformmesh (`self.PlatformMesh`))
  (`StaticMeshComponent.SetStaticMesh` _platformmesh (`self.Static Mesh`))
  (`PrimitiveComponent.SetMaterial` _platformmesh 0 (`self.Material`)))